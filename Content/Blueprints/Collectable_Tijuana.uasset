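; Tijuana collectable that refills the first-person character's second magic ammo pool (Ammo2).
; When destroyed, it adds a fixed increment to Ammo2 if that pool is below the full threshold, with no clamp afterward.
; If the matching magic type is equipped, it also copies the new value into CurrentAmmo.
; The construction script only calls its parent, and no pickup trigger is defined here.
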(event EventDestroyed
  (bind _asfirst_person_character (Utilities|Casting|CastToFirstPersonCharacter (Game|GetPlayerCharacter 0)))
  (if (< (Variables|/Game/FirstPersonBP/Blueprints/FirstPersonCharacter.FirstPersonCharacter_C|GetAmmo2 _asfirst_person_character) 1.0)
    (bind _output_get (Variables|/Game/FirstPersonBP/Blueprints/FirstPersonCharacter.FirstPersonCharacter_C|SetAmmo2 _asfirst_person_character (+ (Variables|/Game/FirstPersonBP/Blueprints/FirstPersonCharacter.FirstPersonCharacter_C|GetAmmo2 _asfirst_person_character) 0.2)))
    (if (Utilities|Enum|Equal(Enum) (Variables|/Game/FirstPersonBP/Blueprints/FirstPersonCharacter.FirstPersonCharacter_C|GetEquippedMagic _asfirst_person_character) "NewEnumerator1")
      (Variables|/Game/FirstPersonBP/Blueprints/FirstPersonCharacter.FirstPersonCharacter_C|SetCurrentAmmo _asfirst_person_character _output_get))))

(fn ConstructionScript
  (|CallParentFunction))