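; Vigor_Spawner_BP is a spawner actor that periodically launches Vigor collectables into the level.
; A looping timer set on BeginPlay fires Spawn, which proceeds only while fewer than five Collectable_Tijuana actors exist.
; It spawns a Collectable_Vigor at its own location with random pitch and yaw, then adds a projectile movement component to it.
; The cap counts Collectable_Tijuana rather than the spawned Collectable_Vigor class.
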(event Custom|Spawn
  (bind _outactors (Actor|GetAllActorsOfClass "/Game/Blueprints/Collectable_Tijuana.Collectable_Tijuana_C"))
  (if (< (Utilities|Array|Length _outactors) 5)
    (bind _returnvalue (Game|SpawnActorfromClass "/Game/Blueprints/Collectable_Vigor.Collectable_Vigor_C" (Math|Transform|MakeTransform (Transformation|GetActorLocation self) (Math|Rotator|MakeRotator 0.0 (Math|Random|RandomFloatinRange 0.0 8e+01) (Math|Random|RandomFloatinRange 0.0 3.6e+02))) "Undefined" 0 0))
    (AddComponent|AddProjectileMovementComponent _returnvalue)))

(event EventBeginPlay
  (Utilities|Time|SetTimerbyEvent (delegate Custom|Spawn) 1e+01 true))

(fn ConstructionScript)