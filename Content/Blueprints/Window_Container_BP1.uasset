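; Window container actor for a breakable greenhouse window that an explosion destroys and magic repairs.
; TriggerExplode fires a radial impulse and marks it broken; TriggerMagic then adds repair progress by magic type, spawning particles on alternate hits.
; At full repair it resets the child Glass actor's destructible mesh and notifies FirstPersonGameMode.
; Focusing a broken window briefly shows a dynamic highlight material driven by repair percentage.
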(event Custom|OnFocus
  (bind _cube (Variables|Default|GetCube))
  ;[1 1 1] Highlight
  (if (Utilities|Enum|Equal(Enum) (Variables|Default|GetState) "NewEnumerator1")
    (Rendering|Material|SetScalarParameterValue (Variables|Default|GetColorChange) "Percentage" (/ (Math|Conversions|ToFloat(Integer) (Variables|Default|GetRepair)) 1e+02) :!class /Script/Engine.MaterialInstanceDynamic)
    (Rendering|Material|SetMaterial _cube 0 (Variables|Default|GetColorChange))
    (Utilities|FlowControl|RetriggerableDelay 0.1)
    (Rendering|Material|SetMaterial _cube 0 "/Game/Blueprints/Materials/Transparent.Transparent")))

(event Custom|TriggerExplode
  ;[1 1 1] Destroy
  (Variables|Default|SetState "NewEnumerator1")
  (Variables|Default|SetRepair 0)
  (Class|RadialForceComponent|FireImpulse (Variables|Default|GetRadialForce)))

(event Custom|TriggerMagic
  (params (Type :type Magic%20Enum :default "NewEnumerator0") (Position :type Vector))
  (bind _returnvalue (Transformation|GetActorRotation))
  (bind _returnvalue_2 (Transformation|GetActorLocation))
  (bind (_roll _pitch _yaw) (Math|Rotator|BreakRotator _returnvalue))
  (bind _returnvalue_3 (- Position _returnvalue_2))
  (bind _returnvalue_4 (Math|Transform|MakeTransform _returnvalue_3 "0, 0, 0" "2.000000,2.000000,2.000000"))
  ;[1 1 1] Interact with window
  (if (Utilities|Enum|Equal(Enum) (Variables|Default|GetState) "NewEnumerator1")
    (switch Utilities|FlowControl|Switch|SwitchonMagic Type
      (:NewEnumerator0
        (if (Variables|Default|GetSpawnParticle)
          (Variables|Default|SetSpawnParticle false)
          ;;[1 1 1] Magic1
          (AddComponent|AddParticleSystemComponent false _returnvalue_4)
          (else
            (Variables|Default|SetSpawnParticle true)))
        (bind _output_get (Variables|Default|SetRepair (+ (Variables|Default|GetRepair) (Variables|Default|GetMagic1)))))
      (:NewEnumerator1
        (if (Variables|Default|GetSpawnParticle)
          (Variables|Default|SetSpawnParticle false)
          ;;[1 1 1] Magic2
          (AddComponent|AddParticleSystemComponent false _returnvalue_4)
          (else
            (Variables|Default|SetSpawnParticle true)))
        (bind _output_get_2 (Variables|Default|SetRepair (+ (Variables|Default|GetRepair) (Variables|Default|GetMagic2))))))
    (if (or (> _output_get 99) (> _output_get_2 99))
      ;;[1 1 1] Rebuild window
      (bind _aswindow_destructible_bp (Utilities|Casting|CastToWindow_Destructible_BP (Variables|/Script/Engine.ChildActorComponent|GetChildActor (Variables|Default|GetGlass))))
      (Class|DestructibleComponent|SetDestructibleMesh (Variables|/Game/Blueprints/Window_Destructible_BP.Window_Destructible_BP_C|GetDestructible _aswindow_destructible_bp) "/Game/art_assets/Evironment/Greenhouse/Greenhouse_Window_DM.Greenhouse_Window_DM")
      (Variables|Default|SetState "NewEnumerator0")
      (bind _asfirst_person_game_mode (Utilities|Casting|CastToFirstPersonGameMode (Game|GetGameMode)))
      (Default|WindowIsRestored _asfirst_person_game_mode self)
      (bind _outactors (Collision|SphereOverlapActors (+ (Class|KismetMathLibrary|CreateVectorfromYawPitch _yaw (+ _pitch 9e+01) 124.0) (Transformation|GetActorLocation) "0,0,50.000000") 5.0 (Utilities|Array|MakeArray "ObjectTypeQuery1") "/Game/Blueprints/Window_Container_BP.Window_Container_BP_C"))
      (for _array_element _outactors
        (Development|PrintString (Utilities|String|ToString(Vector) (Transformation|GetActorLocation _array_element)))))))

(event EventBeginPlay
  (bind _cube (Variables|Default|GetCube))
  ;[1 1 1] Set up
  (Variables|Default|SetState "NewEnumerator0")
  (Variables|Default|SetRepair 0)
  (bind _returnvalue (Rendering|Material|CreateDynamicMaterialInstance _cube 0 "/Game/Blueprints/Materials/Highlight.Highlight" "None" :!class /Script/Engine.PrimitiveComponent))
  (Variables|Default|SetColorChange _returnvalue)
  (Rendering|Material|SetMaterial _cube 0 "/Game/Blueprints/Materials/Transparent.Transparent"))

(fn ConstructionScript)