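; Window container actor that can be shattered and then repaired through repeated player interaction.
; TriggerExplode marks it broken, resets repair progress and fires a radial force impulse.
; TriggerWindow raises progress while broken; at full, it resets the Glass child actor's destructible mesh and restores the initial state.
; OnFocus shows progress on the Cube through a dynamic highlight material, using a retriggerable delay to revert to transparent when focus stops.
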(event Custom|OnFocus
  (bind _cube (Variables|Default|GetCube))
  ;[1 1 1] Highlight
  (if (Utilities|Enum|Equal(Enum) (Variables|Default|GetState) "NewEnumerator1")
    (Rendering|Material|SetScalarParameterValue (Variables|Default|GetColorChange) "Percentage" (/ (Math|Conversions|ToFloat(Integer) (Variables|Default|GetRepair)) 1e+02) :!class /Script/Engine.MaterialInstanceDynamic)
    (Rendering|Material|SetMaterial _cube 0 (Variables|Default|GetColorChange))
    (Utilities|FlowControl|RetriggerableDelay 0.1)
    (Rendering|Material|SetMaterial _cube 0 "/Game/Blueprints/Materials/Transparent.Transparent")))

(event Custom|TriggerExplode
  ;[1 1 1] Destroy
  (Variables|Default|SetState "NewEnumerator1")
  (Variables|Default|SetRepair 0)
  (Class|RadialForceComponent|FireImpulse (Variables|Default|GetRadialForce)))

(event Custom|TriggerWindow
  ;[1 1 1] Interact with window
  (if (Utilities|Enum|Equal(Enum) (Variables|Default|GetState) "NewEnumerator1")
    ;;[1 1 1] Increase repair
    (bind _output_get (Variables|Default|SetRepair (+ (Variables|Default|GetRepair) 1)))
    ;;[1 1 1] Rebuild window
    (if (> _output_get 99)
      (bind _aswindow_destructible_bp (Utilities|Casting|CastToWindow_Destructible_BP (Variables|/Script/Engine.ChildActorComponent|GetChildActor (Variables|Default|GetGlass))))
      (Class|DestructibleComponent|SetDestructibleMesh (Variables|/Game/Blueprints/Window_Destructible_BP.Window_Destructible_BP_C|GetDestructible _aswindow_destructible_bp) "/Game/art_assets/Evironment/Greenhouse/Greenhouse_Window_DM.Greenhouse_Window_DM")
      (Variables|Default|SetState "NewEnumerator0"))))

(event EventBeginPlay
  (bind _cube (Variables|Default|GetCube))
  ;[1 1 1] Set up
  (Variables|Default|SetState "NewEnumerator0")
  (Variables|Default|SetRepair 0)
  (bind _returnvalue (Rendering|Material|CreateDynamicMaterialInstance _cube 0 "/Game/Blueprints/Materials/Highlight.Highlight" "None" :!class /Script/Engine.PrimitiveComponent))
  (Variables|Default|SetColorChange _returnvalue)
  (Rendering|Material|SetMaterial _cube 0 "/Game/Blueprints/Materials/Transparent.Transparent"))

(fn ConstructionScript)